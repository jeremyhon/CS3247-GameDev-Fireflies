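; BP_Firefly is a firefly actor that bobs, glows and can circle a center actor.
; BeginPlay randomizes speed and amplitude, then timelines offset Z around Origin and animate EmissiveStrength on a dynamic material.
; Whirl sets center and radius, and Tick orbits it using sine and cosine, updating Origin.
; Spawn runs a timeline lerping location and Origin toward small random cone vectors, re-rolled each update and not offset by current location.
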(event `self.ReceiveBeginPlay`
  (set `self.isWhirling` false)
  (set `self.timer` 0.0)
  (set `self.speed` (`KismetMathLibrary.RandomFloatInRange` 0.2 0.4))
  (set `self.amplitude` (`KismetMathLibrary.RandomFloatInRange` 20.0 40.0))
  (set `self.origin` (`self.K2_GetActorLocation`))
  (bind (_direction _data) (`Timeline|Vertical Movement` :!via `PlayFromStart`)
    (:`Update`
      (`self.K2_SetActorLocation` (+ (`KismetMathLibrary.MakeVector` 0.0 0.0 (* _data (`self.amplitude`))) (`self.origin`)))
      (bind (_direction_2 _intensity) (`Timeline|IntensityChanger`)
        (:`Update`
          (`MaterialInstanceDynamic.SetScalarParameterValue` (`self.DMI`) "EmissiveStrength" _intensity))))))

(event `self.ReceiveActorBeginOverlap`
  (params (OtherActor :type "Actor Object Reference")))

(event `self.ReceiveTick`
  (params (DeltaSeconds :type "Float (single-precision)"))
  (bind _radius (`self.radius`))
  (bind (_returnvalue_x _returnvalue_y _returnvalue_z) (`KismetMathLibrary.BreakVector` (`self.K2_GetActorLocation` (`self.whirlCenter`))))
  (if (`self.isWhirling`)
    (bind _output_get (set `self.timer` (+ (* DeltaSeconds (`self.speed`)) (`self.timer`))))
    (`self.K2_SetActorLocation` (`KismetMathLibrary.MakeVector` (+ (* (`KismetMathLibrary.Sin` _output_get) _radius) _returnvalue_x) (+ (* _radius (`KismetMathLibrary.Cos` _output_get)) _returnvalue_y) _returnvalue_z))
    (set `self.origin` (`self.K2_GetActorLocation`))))

(event `Whirl`
  (params (center :type "Actor Object Reference"))
  (bind _output_get (set `self.whirlCenter` center))
  (set `self.isWhirling` true)
  (set `self.timer` (/ (`KismetMathLibrary.GetPI`) 2.0))
  (set `self.radius` (`self.GetHorizontalDistanceTo` _output_get)))

(event `Spawn`
  (bind (_direction _alpha) (`Timeline|Movement`)
    (:`Update`
      (bind _returnvalue (`KismetMathLibrary.VLerp` (`self.K2_GetActorLocation`) (* (`KismetMathLibrary.RandomUnitVectorInCone` (0.0 0.0 1.0) 120.0) (`KismetMathLibrary.RandomFloatInRange` 10.0 30.0)) _alpha))
      (`self.K2_SetActorLocation` _returnvalue)
      (set `self.origin` _returnvalue))))

(fn `UserConstructionScript`
  (bind _returnvalue (`PrimitiveComponent.CreateDynamicMaterialInstance` (`self.StaticMesh`) 0 null))
  (set `self.DMI` _returnvalue))